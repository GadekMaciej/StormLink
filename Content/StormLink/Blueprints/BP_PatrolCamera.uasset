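; BP_PatrolCamera is a patrol camera actor that awards score to the player when destroyed by a bullet-time projectile.
; TakeDamage plays a 2D destroy sound for any source, then continues only if the source is BP_SLProjectileBulletTime.
; The projectile's origin perspective selects the first- or third-person score for player 0's state before the actor destroys itself.
; IsCanTakeDamage always returns false, and no patrol logic lives in this graph.
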(event `self.ReceiveBeginPlay`)

(event `self.TakeDamage`
  (params (SourceActor :type "Actor Object Reference") (Instigator :type "Actor Object Reference"))
  (bind _asbp_slplayer_state_base (cast `/Game/StormLink/Blueprints/BP_SLPlayerStateBase` (`Controller.PlayerState` (`GameplayStatics.GetPlayerController` 0)) :!pure true))
  (`GameplayStatics.PlaySound2D` (`self.OnDestroySound`) 1.0 1.0 0.0 null null)
  (bind _asbp_slprojectile_bullet_time (cast `/Game/StormLink/Blueprints/BP_SLProjectileBulletTime` SourceActor))
  (switch `ECameraPerspective` (`/Game/StormLink/Blueprints/BP_SLProjectileBulletTime.OriginPerspective` _asbp_slprojectile_bullet_time)
    (:`FirstPersonPerspective`
      (`/Game/StormLink/Blueprints/BP_SLPlayerStateBase.AddScore` _asbp_slplayer_state_base (`self.FPPScorePrice`)))
    (:`ThirdPersonPerspective`
      (`/Game/StormLink/Blueprints/BP_SLPlayerStateBase.AddScore` _asbp_slplayer_state_base (`self.TPPScorePrice`))))
  (`self.K2_DestroyActor` self))

(event `self.ReceiveDestroyed`
  (`parent.ReceiveDestroyed`))

(fn `IsCanTakeDamage`
  (returns (ReturnValue :type Boolean))
  (return false))

(fn `UserConstructionScript`)