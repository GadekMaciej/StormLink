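; BP_SLCharacterProjectile is a StormLink character projectile that records the perspective its owner had when it began play.
; On BeginPlay it casts its owner to BP_SLCharacterBase and stores CurrentPerspective as OriginPerspective.
; A switch on first or third person only prints a debug string so far.
; The overlap event and construction script just call the parent, and Tick is disabled.
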(event `self.ReceiveBeginPlay`
  (bind (_asbp_slcharacter_base _bsuccess) (cast `/Game/StormLink/Blueprints/BP_SLCharacterBase` (`self.GetOwner`) :!pure true))
  (`parent.ReceiveBeginPlay`)
  (if _bsuccess
    (bind _output_get (set `self.OriginPerspective` (`/Game/StormLink/Blueprints/BP_SLCharacterBase.CurrentPerspective` _asbp_slcharacter_base)))
    (switch `ECameraPerspective` _output_get
      (:`FirstPersonPerspective`
        (`KismetSystemLibrary.PrintString` "1"))
      (:`ThirdPersonPerspective`
        (`KismetSystemLibrary.PrintString` "3")))))

(event `self.ReceiveActorBeginOverlap`
  (params (OtherActor :type "Actor Object Reference"))
  (`parent.ReceiveActorBeginOverlap` OtherActor))

(fn `UserConstructionScript`
  (`parent.UserConstructionScript`))