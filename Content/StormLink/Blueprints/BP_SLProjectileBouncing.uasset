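; BP_SLProjectileBouncing is a StormLink projectile that bounces a limited number of times, damaging DamageTakingEntity actors it bounces off.
; ProjectileMovement bounce events count each bounce and apply damage, then stop simulation once the limit is used up.
; PredictBouncePath forecasts the route with debug-drawn, near-zero-gravity path predictions, mirroring velocity around each impact normal, and stores the last predicted location if the first trace hits.
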(event `self.ProjectileMovement.OnProjectileBounce`
  (params (ImpactResult :type "HitResult Structure (by ref)") (ImpactVelocity :type "Vector Structure (by ref)"))
  (if (< (`self.CurrentNumberOfBounces`) (`self.MaximumNumberOfBounces`))
    (`/Engine/EditorBlueprintResources/StandardMacros.IncrementFloat` (`self.CurrentNumberOfBounces`)
      (:`  `
        (bind _asdamage_taking_entity (cast `DamageTakingEntity` (`.HitActor` (`GameplayStatics.BreakHitResult` ImpactResult))))
        (`DamageTakingEntity.TakeDamage` _asdamage_taking_entity self (`self.GetOwner`))))
    (else
      (`ProjectileMovementComponent.StopSimulating` (`self.ProjectileMovement`) ImpactResult))))

(event `PredictBouncePath`
  (bind _velocity (`MovementComponent.Velocity` (`self.ProjectileMovement`)))
  (set `self.CurrentVelocity` _velocity)
  (bind (_outhit _outpathpositions _outlasttracedestination _returnvalue) (`GameplayStatics.Blueprint_PredictProjectilePath_ByTraceChannel` :`StartPos` (`self.K2_GetActorLocation`) :`LaunchVelocity` _velocity :`ProjectileRadius` (`SphereComponent.SphereRadius` (`self.SphereCollision`)) :`TraceChannel` "ECC_Visibility" :`DrawDebugType` "ForDuration" :`DrawDebugTime` 1.0 :`SimFrequency` 10.0 :`MaxSimTime` 10.0 :`OverrideGravityZ` 0.0001))
  (bind _output_get (set `self.CurrentHit` _returnvalue))
  (if _output_get
    (set `self.CurrentBounceHit` (`|GetArrayItem` _outpathpositions (`KismetArrayLibrary.Array_LastIndex` _outpathpositions)))
    (set `self.CurrentImpactNormal` (`.Normal` (`GameplayStatics.BreakHitResult` _outhit)))
    (set `self.BouncePredictionCount` 0)
    (set `self.CurrentVelocity` (`KismetMathLibrary.MirrorVectorByNormal` (`self.CurrentVelocity`) (`self.CurrentImpactNormal`)) :!label _label)
    (bind _outhit_2 (`GameplayStatics.Blueprint_PredictProjectilePath_ByTraceChannel` :`StartPos` (`self.CurrentBounceHit`) :`LaunchVelocity` (`self.CurrentVelocity`) :`ProjectileRadius` (- (`SphereComponent.SphereRadius` (`self.SphereCollision`)) 10.0) :`TraceChannel` "ECC_WorldStatic" :`DrawDebugType` "ForDuration" :`DrawDebugTime` 1.0 :`SimFrequency` 10.0 :`MaxSimTime` 10.0 :`OverrideGravityZ` 0.0001))
    (bind _output_get_2 (set `self.CurrentHit` (and (< (`self.BouncePredictionCount`) (- (`self.MaximumNumberOfBounces`) 1.0)) (`self.CurrentHit`))))
    (if _output_get_2
      (bind (_bblockinghit _binitialoverlap _time _distance _location _impactpoint _normal) (`GameplayStatics.BreakHitResult` _outhit_2))
      (set `self.CurrentBounceHit` _location)
      (set `self.CurrentImpactNormal` _normal)
      (`/Engine/EditorBlueprintResources/StandardMacros.IncrementInt` (`self.BouncePredictionCount`)
        (:`  `
          (goto _label)))
      (else
        (set `self.LastPredictionLocation` (`self.CurrentBounceHit`))))))

(fn `UserConstructionScript`
  (`parent.UserConstructionScript`))